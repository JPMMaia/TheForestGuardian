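; Base player controller for The Forest Guardian that creates the main HUD on BeginPlay and handles player input.
; Input events forward movement, look, aim, fire, reload, interact and weapon equipping to the possessed C_MainCharacter2, while mouse pitch applies directly to the controller.
; Mouse look only applies when the current input device is Mouse.
; The T key spawns a weapon selection widget, and helpers expose input device, sensitivity and interact key.
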(event EventBeginPlay
  ;[1 1 1] Begin Play
  (bind _returnvalue (UserInterface|CreateWidget "/Game/TheForestGuardian/UserInterface/W_Main.W_Main_C" self (CallFunction|GetMainCharacter)))
  (bind _output_get (Variables|Widgets|SetMainWidget _returnvalue))
  (UserInterface|Viewport|AddtoViewport _output_get 0))

(event Input|ActionEvents|InputActionEquipWeapon1
  (params (Key :type Key%20Structure :default "AnyKey"))
  ;[1 1 1] Equip Weapon
  (:Pressed
    (Default|EquipWeapon (CallFunction|GetMainCharacter) 1)))

(event Input|ActionEvents|InputActionEquipWeapon2
  (params (Key :type Key%20Structure :default "AnyKey"))
  ;[1 1 1] Equip Weapon
  (:Pressed
    (Default|EquipWeapon (CallFunction|GetMainCharacter) 2)))

(event Input|ActionEvents|InputActionEquipWeapon3
  (params (Key :type Key%20Structure :default "AnyKey"))
  ;[1 1 1] Equip Weapon
  (:Pressed
    (Default|EquipWeapon (CallFunction|GetMainCharacter) 3)))

(event Input|ActionEvents|InputActionInteract
  (params (Key :type Key%20Structure :default "AnyKey"))
  ;[1 1 1] Interact
  (:Pressed
    (Variables|Input|SetInteractKey Key)
    (Default|Interact (CallFunction|GetMainCharacter))))

(event Input|ActionEvents|InputActionSwitchAimSide
  (params (Key :type Key%20Structure :default "AnyKey"))
  ;[1 1 1] Switch Aim Side
  (:Pressed
    (Default|SwitchAimSide (CallFunction|GetMainCharacter))))

(event Input|ActionEvents|InputActionShoot
  (params (Key :type Key%20Structure :default "AnyKey"))
  (bind _character (CallFunction|GetMainCharacter))
  ;[1 1 1] Shoot
  (:Pressed
    (Default|Fire _character true))
  (:Released
    (Default|Fire _character false)))

(event Input|ActionEvents|InputActionAim
  (params (Key :type Key%20Structure :default "AnyKey"))
  (bind _character (CallFunction|GetMainCharacter))
  ;[1 1 1] Aim
  (:Pressed
    (Default|Aim _character true))
  (:Released
    (Default|Aim _character false)))

(event Input|ActionEvents|InputActionReload
  (params (Key :type Key%20Structure :default "AnyKey"))
  (bind _character (CallFunction|GetMainCharacter))
  ;[1 1 1] Reload
  (:Pressed
    (if (not (or (Variables|/Game/TheForestGuardian/Blueprints/MainCharacter/C_BaseCharacter2.C_BaseCharacter2_C|GetReloading? _character) (Variables|/Game/TheForestGuardian/Blueprints/MainCharacter/C_BaseCharacter2.C_BaseCharacter2_C|GetIsChangingWeapon _character)))
      (if (not (Default|HaveAmmoinBackpack (Variables|/Game/TheForestGuardian/Blueprints/MainCharacter/C_BaseCharacter2.C_BaseCharacter2_C|GetCurrentWeapon _character)))
        (Default|Reload _character)))))

(event Input|ActionEvents|InputActionWalk
  (params (Key :type Key%20Structure :default "AnyKey"))
  (bind _character (CallFunction|GetMainCharacter))
  (:Pressed
    (Default|Walk _character true))
  (:Released
    (Default|Walk _character false)))

(event Input|AxisEvents|InputAxisTurnRate
  (params (AxisValue :type Float%20%28single-precision%29))
  ;[1 1 1] Turn
  (if (!= AxisValue 0.0)
    (Default|Turn (CallFunction|GetMainCharacter) (* AxisValue (Variables|Input|GetKeyboardTurnSensitivity)))))

(event Input|AxisEvents|InputAxisLookUpRate
  (params (AxisValue :type Float%20%28single-precision%29))
  ;[1 1 1] Look Up
  (if (!= AxisValue 0.0)
    (Default|LookUp (CallFunction|GetMainCharacter) (* AxisValue (Variables|Input|GetKeyboardLookUpSensitivity)))))

(event Input|AxisEvents|InputAxisMoveForward
  (params (AxisValue :type Float%20%28single-precision%29))
  ;[1 1 1] Move Forward
  (if (!= AxisValue 0.0)
    (Default|MoveForward (CallFunction|GetMainCharacter) AxisValue)))

(event Input|AxisEvents|InputAxisMouseX
  (params (AxisValue :type Float%20%28single-precision%29))
  ;[1 1 1] Mouse Axis
  (if (Utilities|Enum|Equal(Enum) (Variables|Input|GetCurrentInputDevice) "NewEnumerator0")
    (Default|Turn (CallFunction|GetMainCharacter) (* AxisValue (Variables|Input|GetMouseSensitivityCurrent)))))

(event Input|AxisEvents|InputAxisMouseY
  (params (AxisValue :type Float%20%28single-precision%29))
  ;[1 1 1] Mouse Axis
  (if (Utilities|Enum|Equal(Enum) (Variables|Input|GetCurrentInputDevice) "NewEnumerator0")
    (Class|PlayerController|AddPitchInput (* AxisValue (Variables|Input|GetMouseSensitivityCurrent)))))

(event Input|KeyboardEvents|T
  (params (Key :type Key%20Structure :default "AnyKey"))
  (:Pressed
    (bind _returnvalue (UserInterface|CreateWidget "/Game/TheForestGuardian/UserInterface/W_WeaponSelection.W_WeaponSelection_C" self))
    (bind _output_get (Variables|Default|SetWeaponWidget _returnvalue))
    (UserInterface|Viewport|AddtoViewport _output_get 0)))

(fn ConstructionScript)

(fn GetCurrentInputDevice
  (return (Variables|Input|GetCurrentInputDevice)))

(fn SetCurrentInputDevice
  (params (NewInputDevice :type E_InputDevice%20Enum))
  (Variables|Input|SetCurrentInputDevice NewInputDevice))

(fn GetSensitivity
  (params (Device :type E_InputDevice%20Enum) (CurrentDevice? :type Boolean))
  (Utilities|FlowControl|Sequence
    (:then_0
      (if CurrentDevice?
        (switch Utilities|FlowControl|Switch|SwitchonE_InputDevice (Variables|Input|GetCurrentInputDevice)
          (:NewEnumerator0
            (LocalVariables|SetLocalSensitivity (Variables|Input|GetMouseSensitivityCurrent))))
        (else
          (switch Utilities|FlowControl|Switch|SwitchonE_InputDevice Device
            (:NewEnumerator0
              (LocalVariables|SetLocalSensitivity (Variables|Input|GetMouseSensitivityCurrent)))))))
    (:then_1
      (return (LocalVariables|GetLocalSensitivity)))))

(fn GetMainCharacter
  (bind _asc_main_character_2 (Utilities|Casting|CastToC_MainCharacter2 (Pawn|GetControlledPawn))
    (:then
      _)
    (:CastFailed
      (Development|PrintString "Failed to cast Controlled Pawn!")))
  (return _asc_main_character_2))

(fn GetInteractKey
  (return (Variables|Input|GetInteractKey)))