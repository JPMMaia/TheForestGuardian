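; Base enemy Blueprint that handles health, incoming weapon damage and death, with an empty MeleeAttack function.
; TakeDamage scales ammo damage by a random weapon modifier, a critical roll and the hit physical material's DestructibleDamageThresholdScale, repurposed as a per-surface multiplier.
; ModifyHealth subtracts the result and refreshes the widget health bar.
; Non-lethal hits spawn a damage feedback actor at the impact point, while lethal ones set a brief lifespan.
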(event EventBeginPlay
  (Variables|Default|SetCurrentHealth (Variables|Default|GetMaxHealth)))

(event EventTakeDamage
  (params (AmmoData :type S%20Ammo%20Data%20Structure) (MinWeaponDamageModifier :type Float%20%28single-precision%29) (MaxWeaponDamageModifier :type Float%20%28single-precision%29) (CriticalDamageModifier :type Float%20%28single-precision%29) (DamageCauser :type Actor%20Object%20Reference) (HitInfo :type Hit%20Result%20Structure))
  (bind (_ammotype _damage _criticalchance) (Utilities|Struct|BreakS_AmmoData AmmoData))
  ;[1 1 1] Take Damage
  (if (not (Variables|Default|GetIsDead))
    (bind (_damagetaken _critical) (CallFunction|CalculateDamage _damage _criticalchance CriticalDamageModifier (Math|Random|RandomFloatinRange MinWeaponDamageModifier MaxWeaponDamageModifier) HitInfo))
    (bind _isdead (CallFunction|ModifyHealth _damagetaken))
    (bind _output_get (Variables|Default|SetIsDead _isdead))
    (if _output_get
      (Actor|SetLifeSpan 0.1)
      (else
        (Game|SpawnActorfromClass "/Game/TheForestGuardian/Blueprints/Objects/Weapons/Damage/A_DamageFeedback.A_DamageFeedback_C" (Math|Transform|MakeTransform (.ImpactPoint (Collision|BreakHitResult HitInfo)) "0, 0, 0" "1,1,1") "AlwaysSpawn" 0 _damagetaken _critical)))))

(fn ConstructionScript)

(fn UpdateHealthBar
  (Default|UpdateHealthBar (.AsW%20Enemy%20Health%20Bar (Utilities|Casting|CastToW_EnemyHealthBar (UserInterface|GetUserWidgetObject (Variables|Default|GetUI_HealthBar)))) (Variables|Default|GetCurrentHealth) (Variables|Default|GetMaxHealth)))

(fn ModifyHealth
  (params (HealthToModify :type Float%20%28single-precision%29))
  (Utilities|FlowControl|Sequence
    (:then_0
      (if (>= HealthToModify (Variables|Default|GetCurrentHealth))
        (LocalVariables|SetLocalIsDead true)
        (Variables|Default|SetCurrentHealth 0.0)
        (else
          (LocalVariables|SetLocalIsDead false)
          (Variables|Default|SetCurrentHealth (- (Variables|Default|GetCurrentHealth) HealthToModify)))))
    (:then_1
      (CallFunction|UpdateHealthBar)
      (return (LocalVariables|GetLocalIsDead)))))

(fn CalculateDamage
  (params (Damage :type Float%20%28single-precision%29) (CriticalChance :type Float%20%28single-precision%29) (CriticalDamageModifier :type Float%20%28single-precision%29) (WeaponDamageModifier :type Float%20%28single-precision%29) (HitInfo :type Hit%20Result%20Structure))
  (LocalVariables|SetLocal_CurrentDamage (* Damage WeaponDamageModifier))
  (Utilities|FlowControl|Sequence
    (:then_0
      (bind _output_get (LocalVariables|SetLocal_Critical (< (Math|Random|RandomFloatinRange 0.0 1e+02) CriticalChance)))
      (if _output_get
        (LocalVariables|SetLocal_CurrentDamage (* (LocalVariables|GetLocal_CurrentDamage) CriticalDamageModifier))))
    (:then_1
      (LocalVariables|SetLocal_CurrentDamage (* (LocalVariables|GetLocal_CurrentDamage) (Variables|/Script/Engine.PhysicalMaterial|GetDestructibleDamageThresholdScale (.PhysMat (Collision|BreakHitResult HitInfo))))))
    (:then_2
      (return (LocalVariables|GetLocal_CurrentDamage) (LocalVariables|GetLocal_Critical)))))

(fn MeleeAttack)