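; C_EnemyWithSword is a sword-wielding enemy character that chases and attacks the player.
; On BeginPlay it spawns an A_Sword, attaches it to the mesh's S_Sword socket and marks it picked.
; Tick steers it straight toward a nearby player with movement input.
; At close range it issues an AI move, jumps and plays the attack montage, gated by IsAttacking; MeleeAttack is empty.
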(event `self.ReceiveBeginPlay`
  (bind _returnvalue (`|SpawnActorFromClass` "/Game/TheForestGuardian/Blueprints/Objects/Weapons/Sword/A_Sword.A_Sword_C" (`self.GetTransform`) "AlwaysSpawn" "OverrideRootScale" self))
  (`self.K2_AttachRootComponentTo` _returnvalue (`self.Mesh`) "S_Sword" "SnapToTarget" false)
  (set `/Game/TheForestGuardian/Blueprints/Objects/A_BaseObject.Picked?` true _returnvalue))

(event `self.MeleeAttack`)

(event `self.ReceiveTick`
  (params (DeltaSeconds :type "Float (single-precision)"))
  (bind _returnvalue (`self.GetDistanceTo` (`GameplayStatics.GetPlayerPawn` 0)))
  (`parent.ReceiveTick` DeltaSeconds)
  (if (`self.IsDead`)
    _
    (elif (<= _returnvalue 3000.0)
      (if (< _returnvalue 200.0)
        (if (not (`self.IsAttacking`))
          (set `self.IsAttacking` true)
          (`AIController.MoveToLocation` (cast `AIController` (`self.GetController`) :!pure true) (`self.K2_GetActorLocation` (`GameplayStatics.GetPlayerPawn` 0)) 200.0 true true false true null true)
          (`KismetSystemLibrary.Delay` 0.1)
          (`self.Jump`)
          (bind _returnvalue_2 (`self.PlayAnimMontage` "/Game/TheForestGuardian/Blueprints/Enemy/AM_EnemyWithSwordAttack.AM_EnemyWithSwordAttack" 1.0 "Default"))
          (`KismetSystemLibrary.Delay` _returnvalue_2)
          (set `self.IsAttacking` false))
        (else
          (`self.AddMovementInput` (`KismetMathLibrary.Normal` (- (`self.K2_GetActorLocation` (`GameplayStatics.GetPlayerPawn` 0)) (`self.K2_GetActorLocation`)))))))))

(fn `UserConstructionScript`
  (`parent.UserConstructionScript`))