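; Player character for The Forest Guardian, a child class adding an orbiting camera, switchable aim shoulder and weapon pickup.
; Each tick the camera pivot follows control rotation, while moving forward or aiming with a weapon snaps the actor to camera yaw.
; A per-tick short camera line trace caches any unpicked base object, which Interact picks up if it is a weapon.
; The TakeDamage override is empty.
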(event `self.ReceiveTick`
  (params (DeltaSeconds :type "Float (single-precision)"))
  ;[1 1 1] Update All
  (`parent.ReceiveTick` DeltaSeconds)
  (`self.UpdateCamera`)
  (`self.UpdatePointedObject`))

(event `/Game/TheForestGuardian/Blueprints/Objects/Weapons/Damage/I_TakeDamage.TakeDamage`
  (params (AmmoData :type "/Game/TheForestGuardian/Blueprints/Objects/Weapons/Ammo/S_AmmoData Structure") (MinWeaponDamageModifier :type "Float (single-precision)") (MaxWeaponDamageModifier :type "Float (single-precision)") (CriticalDamageModifier :type "Float (single-precision)") (DamageCauser :type "Actor Object Reference") (HitInfo :type "HitResult Structure")))

(event `MoveForward`
  (params (ScaleValue :type "Float (double-precision)"))
  ;[1 1 1] Move Forward
  (`self.CenterCharacter`)
  (`self.AddMovementInput` (`KismetMathLibrary.GetForwardVector` (`self.GetControlRotation`)) (select `bool` (`self.IsWalking?`) :`false` ScaleValue :`true` 0.2)))

(event `Turn`
  (params (YawValue :type "Float (double-precision)"))
  ;[1 1 1] Turn
  (`self.AddControllerYawInput` YawValue))

(event `LookUp`
  (params (PitchValue :type "Float (double-precision)"))
  ;[1 1 1] Look Up
  (`self.AddControllerPitchInput` PitchValue))

(event `self.Aim`
  (params (Enable :type Boolean))
  ;[1 1 1] Aim
  (`parent.Aim` Enable)
  (if (`self.WeaponEquipped?`)
    (set `self.bUseControllerRotationYaw` Enable)
    (if Enable
      (`self.CenterCharacter`))))

(fn `CenterCharacter`
  (bind (_returnvalue_roll _returnvalue_pitch) (`KismetMathLibrary.BreakRotator` (`self.K2_GetActorRotation`)))
  (bind _camerapivot (`self.CameraPivot`))
  (bind (_returnvalue_roll_2 _returnvalue_pitch_2 _returnvalue_yaw) (`KismetMathLibrary.BreakRotator` (`SceneComponent.K2_GetComponentRotation` _camerapivot)))
  (bind (_relativerotation_roll _relativerotation_pitch) (`KismetMathLibrary.BreakRotator` (`SceneComponent.RelativeRotation` _camerapivot)))
  (`self.K2_SetActorRelativeRotation` (`KismetMathLibrary.MakeRotator` _returnvalue_roll _returnvalue_pitch _returnvalue_yaw))
  (`SceneComponent.K2_SetRelativeRotation` _camerapivot (`KismetMathLibrary.MakeRotator` _relativerotation_roll _relativerotation_pitch) false false)
  (return))

(fn `GetCurrentSide`
  (returns (NewParam :type "/Game/TheForestGuardian/Blueprints/MainCharacter/E_AimSide Enum"))
  (return (`self.CurrentSide`)))

(fn `GetPointedObject`
  (returns (`Hit Actor` :type "Actor Object Reference") (`Hit?` :type Boolean))
  (return (`self.HitActor`) (`self.Pointing?`)))

(fn `Interact`
  (bind (_hit_actor _hit_) (`self.GetPointedObject`))
  (if _hit_
    (bind _asa_base_weapon (cast `/Game/TheForestGuardian/Blueprints/Objects/Weapons/A_BaseWeapon` _hit_actor))
    (`self.PickObject` _asa_base_weapon)))

(fn `SwitchAimSide`
  (`|ExecutionSequence`
    (:`then_0`
      (set `self.CurrentSide` (select `/Game/TheForestGuardian/Blueprints/MainCharacter/E_AimSide` (`self.CurrentSide`) :`NewEnumerator0` "NewEnumerator1" :`NewEnumerator1` "NewEnumerator0" :!type "/Game/TheForestGuardian/Blueprints/MainCharacter/E_AimSide Enum")))
    (:`then_1`
      (`SceneComponent.K2_SetRelativeLocation` (`self.Camera`) (select `/Game/TheForestGuardian/Blueprints/MainCharacter/E_AimSide` (`self.CurrentSide`) :`NewEnumerator0` (`self.LeftCameraPosition`) :`NewEnumerator1` (`self.RightCameraPosition`)) false false))))

(fn `UpdateCamera`
  (`SceneComponent.K2_SetRelativeRotation` (`self.CameraPivot`) (`KismetMathLibrary.NormalizedDeltaRotator` (`self.GetControlRotation`) (`self.K2_GetActorRotation`)) false false)
  (return))

(fn `UpdatePointedObject`
  (bind _camera (`self.Camera`))
  (bind _returnvalue (`SceneComponent.K2_GetComponentLocation` _camera))
  (bind (_outhit _returnvalue_2) (`KismetSystemLibrary.LineTraceSingleForObjects` _returnvalue (+ _returnvalue (* (`KismetMathLibrary.GetForwardVector` (`SceneComponent.K2_GetComponentRotation` _camera)) 300.0)) (`|MakeArray` "ObjectTypeQuery2" :!type "EObjectTypeQuery Enum")))
  (if _returnvalue_2
    (bind (_bblockinghit _binitialoverlap _time _location _impactpoint _normal _impactnormal _physmat _hitactor) (`GameplayStatics.BreakHitResult` _outhit))
    (bind _asa_base_object (cast `/Game/TheForestGuardian/Blueprints/Objects/A_BaseObject` _hitactor)
      (:`then`
        (if (`/Game/TheForestGuardian/Blueprints/Objects/A_BaseObject.IsPicked?` _asa_base_object)
          _
          (else
            (set `self.Pointing?` true)
            (set `self.HitActor` _hitactor)
            (return))))
      (:`CastFailed`
        _)))
  (set `self.Pointing?` false)
  (set `self.HitActor` null)
  (return))

(fn `UserConstructionScript`
  (`parent.UserConstructionScript`))